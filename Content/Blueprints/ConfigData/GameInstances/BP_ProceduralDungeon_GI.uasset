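; Game instance that builds seeded procedural dungeons from room blueprints; main-menu mode clears and regenerates them in a loop.
; A random stream picks the start room, then timed extensions attach at random endpoints, discarding overlapping rooms.
; Overlapping checkbox actors identify connected endpoints; the rest get caps, then an exit spawns.
; Finally it fits the nav mesh volume to the rooms and randomly gives unused rooms an enemy, chest or nothing.
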(event `/Game/Blueprints/Interfaces/BPI_ProceduralDungeon.InitializeDungeon_IF`
  (`self.VariablesReset`)
  (`self.ProcessSeedInput`)
  (`self.PrintExtensions`)
  (if (`self.ISMainMenu?_GI`)
    (bind _output_get (set `self.BuildDelay` 1.0))
    (`self.GenerateStarterRoom`)
    (`KismetSystemLibrary.Delay` _output_get)
    (`self.Generate Extension Rooms`)
    (else
      (bind _output_get_2 (set `self.BuildDelay` 0.01))
      (`self.GenerateStarterRoom`)
      (`KismetSystemLibrary.Delay` _output_get_2)
      (`self.Generate Extension Rooms`)
      (`self.NavMeshSetup`))))

(event `NavMeshSetup`
  (bind _navmeshref (`self.NavMeshRef`))
  (bind _returnvalue (`GameplayStatics.GetActorOfClass` "/Script/NavigationSystem.NavMeshBoundsVolume"))
  (set `self.NavMeshRef` _returnvalue)
  (bind _outactors (`GameplayStatics.GetAllActorsOfClassWithTag` "/Game/Blueprints/Actors/DungeonRooms/BP_Room_Master.BP_Room_Master_C" "DungeonRoom"))
  (bind _output_get (set `self.AllRooms` _outactors))
  (for _array_element _output_get
    (bind (_origin _boxextent) (`Actor.GetActorBounds` _array_element false false))
    (set `self.NavMeshExtentMinTemp` (- _origin _boxextent))
    (set `self.NavMeshExtentMaxTemp` (+ _origin _boxextent)))
  (set `self.NavMeshCenter` (/ (+ (`self.NavMeshExtentMin`) (`self.NavMeshExtentMax`)) 2.0))
  (set `self.NavMeshTotalSize` (- (`self.NavMeshExtentMax`) (`self.NavMeshExtentMin`)))
  (`Actor.K2_SetActorLocation` _navmeshref (`self.NavMeshCenter`) false false)
  (`Actor.SetActorScale3D` _navmeshref (/ (`self.NavMeshTotalSize`) 200.0))
  (`NavigationSystemV1.OnNavigationBoundsUpdated` (`NavigationSystemV1.GetNavigationSystem`) (`self.NavMeshRef`))
  (`self.RoomRoulette`))

(event `RoomRoulette`
  (bind _seedstream (`self.SeedStream`))
  (bind _unusedrooms (`self.UnusedRooms`))
  (`KismetSystemLibrary.Delay` (`self.BuildDelay`))
  (if (`KismetArrayLibrary.Array_IsEmpty` _unusedrooms)
    (`KismetSystemLibrary.PrintString` "Dungeon Complete" true true (struct :`G` 0.66 :`B` 1.0 :`A` 1.0) 20.0)
    (else
      (set `self.RouletteRoom` (`KismetArrayLibrary.Array_RandomFromStream` _unusedrooms _seedstream))
      (switch `int` (`KismetMathLibrary.RandomIntegerFromStream` _seedstream 3)
        (:`Default`
          (`KismetSystemLibrary.PrintString` "Room Roulette Invalid" true true (struct :`R` 1.0 :`G` 0.04517 :`A` 1.0) 10.0))
        (:`0`
          (`self.GenerateNothing`))
        (:`1`
          (`self.GenerateEnemy`))
        (:`2`
          (`self.GenerateChest`))))))

(event `GenerateNothing`
  (`KismetArrayLibrary.Array_RemoveItem` (`self.UnusedRooms`) (`self.RouletteRoom`))
  (`self.RoomRoulette`))

(event `GenerateEnemy`
  (bind _rouletteroom (`self.RouletteRoom`))
  (`KismetArrayLibrary.Array_RemoveItem` (`self.UnusedRooms`) _rouletteroom)
  (`|SpawnActorFromClass` "/Game/Blueprints/Actors/Characters/Enemies/BP_EnemyCharacter.BP_EnemyCharacter_C" (`SceneComponent.K2_GetComponentToWorld` (`/Game/Blueprints/Actors/DungeonRooms/BP_Room_Master.Forward (local x+)` _rouletteroom)) "Undefined" "MultiplyWithRoot" null null)
  (`self.RoomRoulette`))

(event `GenerateChest`
  (bind _rouletteroom (`self.RouletteRoom`))
  (bind _returnvalue_location (`KismetMathLibrary.BreakTransform` (`SceneComponent.K2_GetComponentToWorld` (`/Game/Blueprints/Actors/DungeonRooms/BP_Room_Master.Forward (local x+)` _rouletteroom))))
  (`KismetArrayLibrary.Array_RemoveItem` (`self.UnusedRooms`) _rouletteroom)
  (`|SpawnActorFromClass` "/Game/Blueprints/Actors/Props/Interactive/BP_ItemChest.BP_ItemChest_C" (`KismetMathLibrary.MakeTransform` _returnvalue_location) "Undefined" "MultiplyWithRoot" null null)
  (`self.RoomRoulette`))

(fn `ClearCurrentDungeon`
  (set `self.LoadingSeed` 0)
  (`KismetArrayLibrary.Array_Clear` (`self.CurrentOverlappedComponents`))
  (`self.VariablesReset`)
  (bind _outactors (`GameplayStatics.GetAllActorsOfClass` "/Game/Blueprints/Actors/DungeonRooms/BP_Room_Master.BP_Room_Master_C"))
  (for _array_element _outactors
    (`Actor.K2_DestroyActor` _array_element))
  (bind _outactors_2 (`GameplayStatics.GetAllActorsOfClass` "/Game/Blueprints/Actors/DungeonRooms/BP_RoomCap.BP_RoomCap_C"))
  (for _array_element_2 _outactors_2
    (`Actor.K2_DestroyActor` _array_element_2))
  (`KismetSystemLibrary.CollectGarbage`))

(fn `Generate Extension Rooms`
  (if (> (`self.Extensions`) 0) :!label _label
    (bind _chosenendpoint (`self.RandomEndpointSelect` (`self.AllEndPoints`)))
    (bind (_chosenextentionclass _chosenextensionindex _endpointtransform) (`self.EndPointCheck` _chosenendpoint)
      (:`ValidEndpoint`
        (bind _returnvalue (`|SpawnActorFromClass` _chosenextentionclass _endpointtransform "Undefined" "MultiplyWithRoot" null null))
        (`self.RoomOverlapCheck` _returnvalue
          (:`GoodRoom`
            (`self.SetUpRoom`)
            (`KismetSystemLibrary.K2_SetTimer` null "Generate Extension Rooms" (`self.BuildDelay`))
            (`KismetSystemLibrary.PrintString` (`KismetStringLibrary.Conv_IntToString` (`self.Extensions`))))
          (:`BadRoom`
            (`Actor.K2_DestroyActor` (`self.CurrentRoom`))
            (goto _label))))
      (:`InvalidEndPoint`
        (`self.ClearCurrentDungeon`) ; FAILSAFE clears current dungeon
        (goto _label)))
    (elif (`self.ISMainMenu?_GI`)
      (`self.ClearCurrentDungeon`)
      (`self.InitializeDungeon_IF`)
      (else
        (`KismetSystemLibrary.PrintString` "Extensions Complete")
        (`self.GenerateEndCheckBoxes`)
        (`self.ProcessValidEndpoints`)
        (`self.GenerateRoomCaps`)
        (`self.CleanupEndCheckboxes`)
        (`self.GenerateExit`)
        (`self.NavMeshSetup`)))))

(fn `GenerateStarterRoom`
  (bind _returnvalue (`|SpawnActorFromClass` (`self.RandomizeStartRoom`) (`self.StartRoomSpawnPoint`) "Undefined" "MultiplyWithRoot" null null)) ; Spawn Start Room
  (set `self.AllEndPoints` (`self.AllEndPoints`))
  (`KismetArrayLibrary.Array_Append` (`self.AllEndPoints`) (`SceneComponent.GetChildrenComponents` (`/Game/Blueprints/Actors/DungeonRooms/BP_Room_Master.EndPoints_Grp` _returnvalue) false))
  (return))

(fn `ProcessSeedInput`
  (bind _loadingseed (`self.LoadingSeed`))
  (bind _seedstream (`self.SeedStream`))
  (bind _seedstream_initialseed (`KismetMathLibrary.BreakRandomStream` (`self.SeedStream`)))
  (if (== _loadingseed 0)
    (`KismetMathLibrary.SeedRandomStream` _seedstream) ; Similar to a variable Setter, but with\nmore functionality.\nThis sets the random seed to be a\nrandom value.
    (set `self.LoadingSeed` _seedstream_initialseed) ; Used as a reference of the seed...
    (else
      (`KismetMathLibrary.SetRandomStreamSeed` _seedstream _loadingseed) ; Also similar to a variable setter\nwith more functionality.\nLooks at the User's inputted number,\nthen sets it as the random seed.
    )))

(fn `RandomizeStartRoom`
  (returns (StartRoomClass :type "/Game/Blueprints/Actors/DungeonRooms/BP_Room_Master Class Reference"))
  (bind _starroomclasses (`self.StarRoomClasses`))
  (return (`|GetArrayItem` _starroomclasses (`KismetMathLibrary.RandomIntegerInRangeFromStream` (`self.SeedStream`) 0 (- (`KismetArrayLibrary.Array_Length` _starroomclasses) 1)))))

(fn `VariablesReset`
  (`KismetArrayLibrary.Array_Clear` (`self.AllEndPoints`))
  (set `self.Extensions` (- (`self.TotalRooms`) 1))
  (set `self.CurrentRoom` null)
  (set `self.StartRoomSpawnPoint` (struct)))